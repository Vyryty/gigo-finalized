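; Service elevator that carries the player between the positions in a floor list, one floor up or down at a time or straight to the lobby.
; Construction wires child button actors to it; moves chain door-close, linear travel and door-open timelines, then update the floor text.
; A trigger box tracks whether the guest's body is inside, gating moves unless a lobby call is absolute; lobby calls skip the Moving check.
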(event `Move Up`
  (bind _returnvalue (+ (`self.CurrentFloor`) 1))
  (if (`self.Player Inside`)
    (if (and (< _returnvalue (`KismetArrayLibrary.Array_Length` (`self.FloorList`))) (not (`self.Moving`)))
      (set `self.Target Floor` _returnvalue)
      (set `self.Moving` true :!label _label)
      (bind (_direction _closedoors) (`Timeline|CloseDoors` :!via `PlayFromStart`)
        (:`Update`
          (`SceneComponent.K2_SetRelativeLocation` (`self.LeftDoor`) (+ (`self.LeftDoorStart`) (* (0.0 -57.0 0.0) _closedoors)) false false)
          (`SceneComponent.K2_SetRelativeLocation` (`self.RightDoor`) (+ (`self.RightDoorStart`) (* (0.0 57.0 0.0) _closedoors)) false false))
        (:`Finished`
          (bind (_direction_2 _elevatormove) (`Timeline|ElevatorMove` :!via `PlayFromStart`)
            (:`Update`
              (`self.K2_SetActorLocation` (`|EaseFunction` "Linear" _elevatormove (`|GetArrayItem` (`self.FloorList`) (`self.CurrentFloor`)) (`|GetArrayItem` (`self.FloorList`) (`self.Target Floor`)))))
            (:`Finished`
              (bind (_direction_3 _opendoors) (`Timeline|OpenDoors` :!via `PlayFromStart`)
                (:`Update`
                  (`SceneComponent.K2_SetRelativeLocation` (`self.LeftDoor`) (+ (`self.LeftDoorStart`) (* (0.0 -57.0 0.0) _opendoors)) false false)
                  (`SceneComponent.K2_SetRelativeLocation` (`self.RightDoor`) (+ (`self.RightDoorStart`) (* (0.0 57.0 0.0) _opendoors)) false false))
                (:`Finished`
                  (set `self.Moving` false)
                  (bind _output_get (set `self.CurrentFloor` (`self.Target Floor`)))
                  (bind _output_get_2 (set `self.Level` (`KismetStringLibrary.Conv_IntToString` (+ _output_get 1))))
                  (`TextRenderComponent.K2_SetText` (`self.TextRender`) (`KismetTextLibrary.Conv_StringToText` _output_get_2)))))))))))

(event `Move Down`
  (bind _returnvalue (- (`self.CurrentFloor`) 1))
  (if (`self.Player Inside`)
    (if (and (>= _returnvalue 0) (not (`self.Moving`)))
      (set `self.Target Floor` _returnvalue)
      (goto _label))))

(event `Move Lobby`
  (params (Absolute :type Boolean))
  (if (and (!= (`self.CurrentFloor`) 0) (or Absolute (`self.Player Inside`)))
    (set `self.Target Floor` 0)
    (goto _label)))

(event `self.Box.OnComponentBeginOverlap`
  (params (OverlappedComponent :type "PrimitiveComponent Object Reference") (OtherActor :type "Actor Object Reference") (OtherComp :type "PrimitiveComponent Object Reference") (OtherBodyIndex :type Integer) (bFromSweep :type Boolean) (SweepResult :type "HitResult Structure (by ref)"))
  (cast `/Game/Blueprints/BP_JohnGuest` OtherActor)
  (if (`ActorComponent.ComponentHasTag` OtherComp "Body")
    (set `self.Player Inside` true)))

(event `self.Box.OnComponentEndOverlap`
  (params (OverlappedComponent :type "PrimitiveComponent Object Reference") (OtherActor :type "Actor Object Reference") (OtherComp :type "PrimitiveComponent Object Reference") (OtherBodyIndex :type Integer))
  (cast `/Game/Blueprints/BP_JohnGuest` OtherActor)
  (if (`ActorComponent.ComponentHasTag` OtherComp "Body")
    (set `self.Player Inside` false)))

(fn `Interact`
  (params (Interactor :type "Actor Object Reference"))
  (returns (Success :type Boolean))
  (return true))

(fn `UserConstructionScript`
  (`parent.UserConstructionScript`)
  (`|ExecutionSequence`
    (:`then_0`
      (bind _asbp_elevator_button (cast `/Game/Blueprints/BP_ElevatorButton` (`ChildActorComponent.ChildActor` (`self.UpButton`))))
      (set `/Game/Blueprints/BP_ElevatorButton.Elevator` self _asbp_elevator_button)
      (set `/Game/Blueprints/BP_ElevatorButton.isUp` true _asbp_elevator_button)
      (`PrimitiveComponent.SetMaterial` (`/Game/Blueprints/BP_ElevatorButton.PhysicalButton` _asbp_elevator_button) 0 "/Game/Materials/Elevator_Textures/Buttons/Up/Up_Button_mt.Up_Button_mt"))
    (:`then_1`
      (bind _asbp_elevator_button_2 (cast `/Game/Blueprints/BP_ElevatorButton` (`ChildActorComponent.ChildActor` (`self.DownButton`))))
      (set `/Game/Blueprints/BP_ElevatorButton.Elevator` self _asbp_elevator_button_2)
      (set `/Game/Blueprints/BP_ElevatorButton.isUp` false _asbp_elevator_button_2)
      (`PrimitiveComponent.SetMaterial` (`/Game/Blueprints/BP_ElevatorButton.PhysicalButton` _asbp_elevator_button_2) 0 "/Game/Materials/Elevator_Textures/Buttons/Down/Down_Button_mt.Down_Button_mt"))
    (:`then_2`
      (bind _asbp_lobby_button (cast `/Game/Blueprints/BP_LobbyButton` (`ChildActorComponent.ChildActor` (`self.LobbyButton`))))
      (set `/Game/Blueprints/BP_LobbyButton.Elevator` self _asbp_lobby_button))
    (:`then_3`
      (set `self.RightDoorStart` (`SceneComponent.RelativeLocation` (`self.RightDoor`)))
      (set `self.LeftDoorStart` (`SceneComponent.RelativeLocation` (`self.LeftDoor`))))))