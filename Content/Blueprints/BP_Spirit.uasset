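; BP_Spirit is a ghost enemy that periodically panics every guest in its target room while alive.
; A camera-flash reaction stuns it, freezing its animation and pausing the scare timer.
; When damaged while not stunned, it turns toward the player and attacks overlap-tracked "Body" targets, hurting BP_JohnGuest and panicking other guests.
; On defeat it plays a vanish animation and sound, then destroys itself after a delay.
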(event `self.ReceiveBeginPlay`
  (`parent.ReceiveBeginPlay`))

(event `self.ReceiveTick`
  (params (DeltaSeconds :type "Float (single-precision)"))
  (bind _stunned_timer (`self.Stunned Timer`))
  (bind _boo_timer (`self.Boo Timer`))
  (`parent.ReceiveTick` DeltaSeconds)
  (if (`self.Alive`)
    (if (> _stunned_timer 0.0)
      (set `self.Stunned Timer` (- _stunned_timer DeltaSeconds))
      (set `self.Was Stunned` true)
      (else
        (`|ExecutionSequence`
          (:`then_0`
            (if (`self.Was Stunned`)
              (set `self.Was Stunned` false)
              (`SkeletalMeshComponent.PlayAnimation` (`self.Ghost Skeleton`) "/Game/Models/Ghosts/Spirit_Character/Animations/Anim_Spirit_Idle.Anim_Spirit_Idle" true)))
          (:`then_1`
            (if (> _boo_timer 0.0)
              (set `self.Boo Timer` (- _boo_timer DeltaSeconds))
              (else
                (`self.Scare Guests`)))))))))

(event `self.Attack Range.OnComponentBeginOverlap`
  (params (OverlappedComponent :type "PrimitiveComponent Object Reference") (OtherActor :type "Actor Object Reference") (OtherComp :type "PrimitiveComponent Object Reference") (OtherBodyIndex :type Integer) (bFromSweep :type Boolean) (SweepResult :type "HitResult Structure (by ref)"))
  (if (`ActorComponent.ComponentHasTag` OtherComp "Body")
    (`BlueprintSetLibrary.Set_Add` (`self.Targets`) OtherActor)))

(event `self.Attack Range.OnComponentEndOverlap`
  (params (OverlappedComponent :type "PrimitiveComponent Object Reference") (OtherActor :type "Actor Object Reference") (OtherComp :type "PrimitiveComponent Object Reference") (OtherBodyIndex :type Integer))
  (if (`ActorComponent.ComponentHasTag` OtherComp "Body")
    (`BlueprintSetLibrary.Set_Remove` (`self.Targets`) OtherActor)))

(event `Animate Attack`
  (bind _ghost_skeleton (`self.Ghost Skeleton`))
  (`SkeletalMeshComponent.PlayAnimation` _ghost_skeleton "/Game/Models/Ghosts/Spirit_Character/Animations/Anim_Spirit_Attack.Anim_Spirit_Attack" false)
  (`KismetSystemLibrary.Delay` 1.5)
  (if (`self.Alive`)
    (`SkeletalMeshComponent.PlayAnimation` _ghost_skeleton "/Game/Models/Ghosts/Spirit_Character/Animations/Anim_Spirit_Idle.Anim_Spirit_Idle" true)))

(fn `Attack`
  (bind _result (`BlueprintSetLibrary.Set_ToArray` (`self.Targets`)))
  (for _array_element _result
    (bind _asbp_john_guest (cast `/Game/Blueprints/BP_JohnGuest` _array_element)
      (:`then`
        (`/Game/Blueprints/BP_JohnGuest.On Damage` _asbp_john_guest null 0.3))
      (:`CastFailed`
        (bind _asbp_guest (cast `/Game/Blueprints/BP_Guest` _array_element))
        (`/Game/Blueprints/BP_Guest.Induce Panic` _asbp_guest 1.0))))
  (`self.Animate Attack`))

(fn `Flash Cam React`
  (set `self.Stunned Timer` (`self.Stunned Time`))
  (`SkeletalMeshComponent.Stop` (`self.Ghost Skeleton`)))

(fn `Get Locomotiveness`
  (returns (Locomotiveness :type "Float (double-precision)"))
  (return (`self.Locomotiveness`)))

(fn `On Damage`
  (bind _ghost_skeleton (`self.Ghost Skeleton`))
  (if (<= (`self.Stunned Timer`) 0.0)
    (bind _player_ref (`/Game/Blueprints/BP_GIGO_GameMode.Player Ref` (`self.Gamemode Ref`))
      (:`then`
        (bind (_returnvalue_roll _returnvalue_pitch _returnvalue_yaw) (`KismetMathLibrary.BreakRotator` (`KismetMathLibrary.FindLookAtRotation` (`SceneComponent.GetForwardVector` _ghost_skeleton) (- (`SceneComponent.K2_GetComponentLocation` (`Character.CapsuleComponent` _player_ref)) (`SceneComponent.K2_GetComponentLocation` _ghost_skeleton)))))
        (`SceneComponent.K2_SetWorldRotation` _ghost_skeleton (`KismetMathLibrary.MakeRotator` 0.0 0.0 (+ _returnvalue_yaw -90.0)) false false)
        (`self.Attack`))
      (:`else`))))

(fn `On Defeat`
  (`SkeletalMeshComponent.PlayAnimation` (`self.Ghost Skeleton`) "/Game/Models/Ghosts/Spirit_Character/Animations/Anim_Spirit_Vanish.Anim_Spirit_Vanish" false)
  (`self.Play Sound` "/Game/Audio/Ghost_Defeat_1.Ghost_Defeat_1")
  (`self.Destroy After Delay` 5.0))

(fn `Scare Guests`
  (set `self.Boo Timer` (`self.Boo Time`))
  (bind _result (`BlueprintSetLibrary.Set_ToArray` (`/Game/Blueprints/BP_Room.Guest Set` (`self.Target Room`))))
  (for _array_element _result
    (`/Game/Blueprints/BP_Guest.Induce Panic` _array_element 1.0)))

(fn `UserConstructionScript`
  (`parent.UserConstructionScript`)
  (set `self.Boo Timer` (`self.Boo Time`)))