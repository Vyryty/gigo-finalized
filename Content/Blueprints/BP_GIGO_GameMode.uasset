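; Game mode for a haunted-hotel game, running each night from main menu to victory at time-out or defeat at full panic.
; Reset scales guest count and spawn economy by difficulty, spawns guests and plays a one-time cutscene.
; Tick advances the clock and accrues spawn coins, spent by chance rolls on enemies in clusters of nearby hauntable rooms.
; It also manages lobby music, the highlight post-process volume and end-of-night cleanup.
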(event `self.ReceiveBeginPlay`
  (set `self.Rooms` (`self.Get Rooms`))
  ;[0.1198 0.1198 0.1198] For Highlighting
  (bind _returnvalue (`|SpawnActorFromClass` (`self.PPV Class Reference`) (`KismetMathLibrary.MakeTransform` (0.0 0.0 0.0)) "Undefined" "MultiplyWithRoot" null null))
  (set `PostProcessVolume.bUnbound` true _returnvalue)
  (setmembers `PostProcessSettings` :`StructRef` (`PostProcessVolume.Settings` _returnvalue) :`WeightedBlendables` (make `WeightedBlendables` (`|MakeArray` (make `WeightedBlendable` 1.0 "/Game/Materials/HighlightMat.HighlightMat"))))
  (`|ExecutionSequence`
    (:`then_0`
      (bind _outactors (`GameplayStatics.GetAllActorsOfClass` "/Game/Blueprints/BP_JohnGuest.BP_JohnGuest_C"))
      (bind _output_get (set `self.Player Ref` (`|GetArrayItem` _outactors)))
      (`/Engine/EditorBlueprintResources/StandardMacros.IsValid` _output_get
        (:`Is Valid`
          (`/Game/Blueprints/BP_JohnGuest.Set Main Menu Mode` _output_get "/Game/Widgets/WG_MainMenu.WG_MainMenu_C"))))
    (:`then_1`
      (bind _outactors_2 (`GameplayStatics.GetAllActorsOfClass` "/Game/Blueprints/BP_GuestElevator.BP_GuestElevator_C"))
      (set `self.Guest Elevators` _outactors_2))
    (:`then_2`
      (bind _outactors_3 (`GameplayStatics.GetAllActorsOfClass` "/Game/Blueprints/BP_ServiceElevator.BP_ServiceElevator_C"))
      (set `self.Service Elevators` _outactors_3))
    (:`then_3`
      (bind _outactors_4 (`GameplayStatics.GetAllActorsOfClass` "/Script/Engine.PlayerStart"))
      (set `self.Respawn Transform` (`self.GetTransform` (`|GetArrayItem` _outactors_4))))
    (:`then_4`
      (bind _outactors_5 (`GameplayStatics.GetAllActorsOfClass` "/Game/Blueprints/BP_LobbySpeaker.BP_LobbySpeaker_C"))
      (bind _output_get_2 (set `self.Lobby Speakers` _outactors_5))
      (if (<= (`KismetArrayLibrary.Array_Length` _output_get_2) 0)
        (bind _returnvalue_2 (`|SpawnActorFromClass` "/Game/Blueprints/BP_LobbySpeaker.BP_LobbySpeaker_C" (`KismetMathLibrary.MakeTransform` (0.0 0.0 0.0)) "Undefined" "MultiplyWithRoot" null null))
        (`KismetArrayLibrary.Array_Add` (`self.Lobby Speakers`) _returnvalue_2)))
    (:`then_5`
      (bind _outactor (`LevelSequencePlayer.CreateLevelSequencePlayer` "/Game/Animation/Anim_Cutscene.Anim_Cutscene"))
      (set `self.Cutscene Obj` _outactor))))

(event `Reset`
  (set `self.Panic` 0.0)
  (set `self.Time` 0.0)
  (set `self.Spawn Coins` 0)
  (set `self.SC Tracker` 0)
  (set `self.Spawn Coin Timer` (`self.Spawn Coin Rate`))
  (`self.Determine Difficulty Stats`)
  (`self.Spawn Guests`)
  (bind _asbp_gigo_game_instance (cast `/Game/Blueprints/BP_GIGO_GameInstance` (`GameplayStatics.GetGameInstance`))
    (:`then`
      (if (not (`/Game/Blueprints/BP_GIGO_GameInstance.Played Cutscene` _asbp_gigo_game_instance))
        (set `/Game/Blueprints/BP_GIGO_GameInstance.Played Cutscene` true _asbp_gigo_game_instance)
        (bind _cutscene_obj (`self.Cutscene Obj` :!label _label)
          (:`then`
            (bind _player_ref (`self.Player Ref`)
              (:`then`
                (set `/Game/Blueprints/BP_JohnGuest.Can Input` false _player_ref))
              (:`else`
                _))
            (bind _sequenceplayer (`LevelSequenceActor.SequencePlayer` _cutscene_obj))
            (`MovieSceneSequencePlayer.Play` _sequenceplayer)
            (`KismetSystemLibrary.Delay` (`TimeManagementBlueprintLibrary.Conv_QualifiedFrameTimeToSeconds` (`MovieSceneSequencePlayer.GetDuration` _sequenceplayer)))
            (`MovieSceneSequencePlayer.Stop` _sequenceplayer))
          (:`else`
            _))))
    (:`CastFailed`
      (goto _label)))
  (set `self.Game Started` true)
  (`self.Replay Song`)
  (bind _player_ref_2 (`self.Player Ref`)
    (:`then`
      (set `/Game/Blueprints/BP_JohnGuest.Can Input` true _player_ref_2))
    (:`else`)))

(event `self.ReceiveTick`
  (params (DeltaSeconds :type "Float (single-precision)"))
  (bind _song_length (`self.Song Length`))
  (bind _spawn_coin_timer (`self.Spawn Coin Timer`))
  (bind _night_length (`self.Night Length`))
  (if (`self.Game Started`)
    (`|ExecutionSequence`
      (:`then_0`
        (bind _output_get (set `self.Time` (`KismetMathLibrary.FClamp` (+ (`self.Time`) DeltaSeconds) 0.0 _night_length)))
        (if (< _output_get _night_length)
          (if (< _spawn_coin_timer (`self.Spawn Coin Rate`))
            (set `self.Spawn Coin Timer` (+ _spawn_coin_timer DeltaSeconds))
            (else
              (set `self.Spawn Coin Timer` 0.0)
              (set `self.Spawn Coins` (`KismetMathLibrary.Clamp` (+ (`self.Spawn Coins`) 1) 0 (`self.Max Spawn Coins`)))
              (set `self.SC Tracker` (mod (+ (`self.SC Tracker`) 1) (`KismetMathLibrary.Max` (`self.Modded Wallet`) 1)))
              (`self.Roll For Enemy`)))
          (else
            (`self.On Win Night`))))
      (:`then_1`
        (if (`self.Music Playing`)
          (bind _output_get_2 (set `self.Song Time` (`KismetMathLibrary.FClamp` (+ DeltaSeconds (`self.Song Time`)) 0.0 _song_length)))
          (if (>= _output_get_2 _song_length)
            (set `self.Music Playing` false)))))))

(fn `Change Panic`
  (params (Amount :type "Float (double-precision)"))
  (bind _output_get (set `self.Panic` (`KismetMathLibrary.FClamp` (+ Amount (`self.Panic`)))))
  (if (>= _output_get 1.0)
    (`self.On Lose Game` true)))

(fn `Determine Difficulty Stats`
  (locals (LCM :type Integer))
  (bind _lcm (`local.LCM`))
  (bind _returnvalue (- (`BlueprintMapLibrary.Map_Length` (`self.Rooms`)) 1))
  (for _array_element (`self.Enemy Types`)
    (set `local.LCM` (+ (`.EnemyCost_6_AEB470A84EAF06244BBA44BEBE2B8A05` (break `/Game/Blueprints/BP_EnemySpawnData` _array_element)) _lcm)))
  (set `self.Modded Wallet` _lcm)
  (bind _asbp_gigo_game_instance (cast `/Game/Blueprints/BP_GIGO_GameInstance` (`GameplayStatics.GetGameInstance`)))
  (bind _difficulty (`/Game/Blueprints/BP_GIGO_GameInstance.Get Difficulty` _asbp_gigo_game_instance))
  (`KismetSystemLibrary.PrintString` (`KismetStringLibrary.Concat_StrStr` "Difficulty: " (`KismetStringLibrary.Conv_IntToString` _difficulty) ", Night: " (`KismetStringLibrary.Conv_IntToString` (`/Game/Blueprints/BP_GIGO_GameInstance.Current Night` _asbp_gigo_game_instance))))
  (set `self.Max Spawn Coins` (* _difficulty 5))
  (set `self.Spawn Coin Rate` (`KismetMathLibrary.SelectFloat` (`self.Night Length`) (+ (`KismetMathLibrary.MultiplyMultiply_FloatFloat` 5.0 (+ (* _difficulty -0.2) 1.1)) 0.75) (<= _difficulty 0)))
  (set `self.Guest Count` (`KismetMathLibrary.FTrunc` (`KismetMathLibrary.Lerp` (* _returnvalue 0.1) (`KismetMathLibrary.Conv_IntToDouble` _returnvalue) (`KismetMathLibrary.SelectFloat` 0.2 (`KismetMathLibrary.FClamp` (/ _difficulty (`KismetMathLibrary.FMax` 10.0 1.0))) (<= _difficulty 0))))))

(fn `Get Adjacent Hauntable Rooms`
  (params (`Room Name` :type String) (Count :type Integer) (`Max Distance` :type "Float (double-precision)"))
  (returns (`Adjacent Rooms` :type "Array of /Game/Blueprints/BP_Room Object Reference"))
  (locals (`Current Room Number` :type Integer) (`Minimum Floor Number` :type Integer :default 1) (`Maximum Floor Number` :type Integer :default 18) (Increasing :type Boolean :default false) (Result :type "Array of /Game/Blueprints/BP_Room Object Reference") (Distances :type "Array of Float (double-precision)"))
  (bind _result (`local.Result`))
  (bind (_value _returnvalue) (`BlueprintMapLibrary.Map_Find` (`self.Rooms`) `Room Name`))
  (bind (_x _y) (`KismetMathLibrary.BreakVector3f` (* (1.0 1.0 0.0) `Max Distance`)))
  (`|ExecutionSequence`
    (:`then_0`
      (if _returnvalue
        (bind _outactors (`KismetSystemLibrary.BoxOverlapActors` (`SceneComponent.K2_GetComponentLocation` (`/Game/Blueprints/BP_Room.DefaultSceneRoot` _value)) (`KismetMathLibrary.MakeVector` _x _y 100.0) (`|MakeArray` "ObjectTypeQuery1" "ObjectTypeQuery2" "ObjectTypeQuery4" :!type "EObjectTypeQuery Enum") "/Game/Blueprints/BP_Room.BP_Room_C" (`|MakeArray` _value :!type "Actor Object Reference")))
        (for _array_element _outactors
          (if (< (`KismetArrayLibrary.Array_Length` _result) Count)
            (bind _asbp_room (cast `/Game/Blueprints/BP_Room` _array_element))
            (if (`/Game/Blueprints/BP_Room.Can Haunt` _asbp_room)
              (`KismetArrayLibrary.Array_Add` _result _asbp_room))
            (else
              (break))))))
    (:`then_1`
      (return (`local.Result`)))))

(fn `Get Cameras`
  (returns (`Camera Dictionary` :type "Map of String to /Game/Blueprints/BP_Camera Object Reference"))
  (bind _cameras (`self.Cameras`))
  (if (`BlueprintMapLibrary.Map_IsEmpty` (`self.Cameras`))
    (bind _outactors (`GameplayStatics.GetAllActorsOfClass` "/Game/Blueprints/BP_Camera.BP_Camera_C"))
    (for _array_element _outactors
      (bind _keys (`BlueprintMapLibrary.Map_Keys` _cameras))
      (`BlueprintMapLibrary.Map_Add` _cameras (`self.Get Unique Name` (`/Game/Blueprints/BP_Camera.Name` _array_element) _keys) _array_element)))
  (return _cameras))

(fn `Get Clock Time`
  (returns (`Clock Time` :type String))
  (bind _returnvalue (+ (* (`self.Starting Time`) 60.0) (`self.Time`)))
  (bind _returnvalue_2 (/ (`self.Night Length`) (`KismetMathLibrary.FMax` (`self.In Game Hours`) 1.0)))
  (bind _returnvalue_3 (* _returnvalue_2 12.0))
  (bind _returnvalue_4 (`KismetMathLibrary.FFloor` (mod (/ _returnvalue (`KismetMathLibrary.FMax` _returnvalue_2 0.001)) _returnvalue_3)))
  (return (`KismetStringLibrary.Concat_StrStr` (`KismetStringLibrary.Conv_IntToString` (`KismetMathLibrary.SelectInt` 12 _returnvalue_4 (== _returnvalue_4 0))) (`KismetMathLibrary.SelectString` ":00 AM" ":00 PM" (< _returnvalue _returnvalue_3)))))

(fn `Get Hauntable Cluster`
  (params (`Cluster Size` :type Integer) (`Cluster Max Dist` :type "Float (double-precision)"))
  (returns (Rooms :type "Array of /Game/Blueprints/BP_Room Object Reference"))
  (locals (Index :type Integer) (`Random Attempts` :type Integer) (Succeeded :type Boolean) (Result :type "Array of /Game/Blueprints/BP_Room Object Reference"))
  (bind _rooms (`self.Rooms`))
  (bind _keys (`BlueprintMapLibrary.Map_Keys` _rooms))
  (bind _returnvalue (`KismetArrayLibrary.Array_Length` _keys))
  (while (and (not (`local.Succeeded`)) (< (`local.Random Attempts`) (* _returnvalue 2)))
    (`/Engine/EditorBlueprintResources/StandardMacros.IncrementInt` (`local.Random Attempts`)
      (:`  `
        (bind _output_get (set `local.Index` (`KismetMathLibrary.FTrunc` (* _returnvalue (`KismetMathLibrary.RandomFloat`)))))
        (set `local.Succeeded` (`/Game/Blueprints/BP_Room.Can Haunt` (`BlueprintMapLibrary.Map_Find` _rooms (`|GetArrayItem` _keys _output_get)))))))
  (if (not (`local.Succeeded`))
    (for (_array_element _array_index) _keys
      (set `local.Index` _array_index)
      (if (`/Game/Blueprints/BP_Room.Can Haunt` (`BlueprintMapLibrary.Map_Find` _rooms _array_element))
        (set `local.Succeeded` true)
        (break)))
    (if (`local.Succeeded`)
      (bind _output (`|GetArrayItem` _keys (`local.Index`)))
      (bind _output_get_2 (set `local.Result` (`self.Get Adjacent Hauntable Rooms` _output `Cluster Size` `Cluster Max Dist`) :!label _label))
      (`KismetArrayLibrary.Array_Add` _output_get_2 (`BlueprintMapLibrary.Map_Find` _rooms _output)))
    (else
      (goto _label)))
  (return (`local.Result`)))

(fn `Get Panic`
  (returns (Panic :type "Float (double-precision)"))
  (return (`self.Panic`)))

(fn `Get Random Habitable Room`
  (returns (Rooms :type "/Game/Blueprints/BP_Room Object Reference"))
  (locals (Index :type Integer) (`Random Attempts` :type Integer) (Succeeded :type Boolean))
  (bind _rooms (`self.Rooms`))
  (bind _keys (`BlueprintMapLibrary.Map_Keys` _rooms))
  (`KismetArrayLibrary.Array_RemoveItem` _keys "Lobby")
  (bind _returnvalue (`KismetArrayLibrary.Array_Length` _keys))
  (while (and (not (`local.Succeeded`)) (< (`local.Random Attempts`) (* _returnvalue 2)))
    (`/Engine/EditorBlueprintResources/StandardMacros.IncrementInt` (`local.Random Attempts`)
      (:`  `
        (bind _output_get (set `local.Index` (`KismetMathLibrary.FTrunc` (* _returnvalue (`KismetMathLibrary.RandomFloat`)))))
        (set `local.Succeeded` (`/Game/Blueprints/BP_Room.Available For Guests` (`BlueprintMapLibrary.Map_Find` _rooms (`|GetArrayItem` _keys _output_get)))))))
  (if (not (`local.Succeeded`))
    (for (_array_element _array_index) _keys
      (set `local.Index` _array_index)
      (if (`/Game/Blueprints/BP_Room.Available For Guests` (`BlueprintMapLibrary.Map_Find` _rooms _array_element))
        (set `local.Succeeded` true)
        (break))))
  (if (`local.Succeeded`)
    (return (`BlueprintMapLibrary.Map_Find` _rooms (`|GetArrayItem` _keys (`local.Index`))))
    (else
      (return null))))

(fn `Get Rooms`
  (returns (`Camera Dictionary` :type "Map of String to /Game/Blueprints/BP_Room Object Reference"))
  (locals (Result :type "Map of String to /Game/Blueprints/BP_Room Object Reference"))
  (bind _result (`local.Result`))
  (bind _outactors (`GameplayStatics.GetAllActorsOfClass` "/Game/Blueprints/BP_Room.BP_Room_C"))
  (for _array_element _outactors
    (bind _keys (`BlueprintMapLibrary.Map_Keys` _result))
    (`BlueprintMapLibrary.Map_Add` _result (`self.Get Unique Name` (`/Game/Blueprints/BP_Room.Room Name` _array_element) _keys) _array_element))
  (return _result))

(fn `Get Time`
  (returns (Time :type "Float (double-precision)"))
  (return (`self.Time`)))

(fn `Get Unique Name`
  (params (`Current Name` :type String) (`Taken Names` :type "Array of String"))
  (returns (`Unique Name` :type String))
  (bind _returnvalue (- (`KismetStringLibrary.Len` `Current Name`) 1))
  (bind _returnvalue_2 (`KismetStringLibrary.GetSubstring` `Current Name` _returnvalue))
  (if (`KismetArrayLibrary.Array_Contains` `Taken Names` `Current Name`)
    (return (`KismetMathLibrary.SelectString` (`KismetStringLibrary.Concat_StrStr` (`KismetStringLibrary.GetSubstring` `Current Name` 0 _returnvalue) (`KismetStringLibrary.Conv_IntToString` (+ (`KismetStringLibrary.Conv_StringToInt` _returnvalue_2) 1))) (`KismetStringLibrary.Concat_StrStr` `Current Name` " 1") (`KismetStringLibrary.IsNumeric` _returnvalue_2)))
    (else
      (return `Current Name`))))

(fn `On End Game`
  (bind (_respawn_transform_location _respawn_transform_rotation) (`KismetMathLibrary.BreakTransform` (`self.Respawn Transform`)))
  (bind _ghosts (`self.Ghosts`))
  (bind _guests (`self.Guests`))
  (`|ExecutionSequence`
    (:`then_0`
      (bind _player_ref (`self.Player Ref`)
        (:`then`
          (`/Game/Blueprints/BP_JohnGuest.Restart` _player_ref)
          (`SceneComponent.K2_SetWorldLocation` (`Character.CapsuleComponent` _player_ref) _respawn_transform_location false false)
          (bind _asplayer_controller (cast `PlayerController` (`Pawn.GetController` _player_ref)))
          (`Controller.SetControlRotation` _asplayer_controller _respawn_transform_rotation))
        (:`else`)))
    (:`then_1`
      (for _array_element (`self.Service Elevators`)
        (`/Game/Blueprints/BP_ServiceElevator.Move Lobby` _array_element true))
      (for _array_element_2 _ghosts
        (`self.K2_DestroyActor` _array_element_2))
      (`KismetArrayLibrary.Array_Clear` _ghosts)
      (for _array_element_3 _guests
        (`self.K2_DestroyActor` _array_element_3))
      (`KismetArrayLibrary.Array_Clear` _guests)
      (bind _values (`BlueprintMapLibrary.Map_Values` (`self.Rooms`)))
      (for _array_element_4 _values
        (set `/Game/Blueprints/BP_Room.Heated` false _array_element_4))
      (for _array_element_5 (`self.Lobby Speakers`)
        (`AudioComponent.SetPaused` (`/Game/Blueprints/BP_LobbySpeaker.Speaker` _array_element_5) true)))))

(fn `On Lose Game`
  (params (Panicked :type Boolean))
  (set `self.Game Started` false)
  (`self.On End Game`)
  (bind _player_ref (`self.Player Ref`)
    (:`then`
      (`/Game/Blueprints/BP_JohnGuest.Set Main Menu Mode` _player_ref "/Game/Widgets/WG_Defeat.WG_Defeat_C"))
    (:`else`)))

(fn `On Win Night`
  (set `self.Game Started` false)
  (`self.On End Game`)
  (bind _player_ref (`self.Player Ref`)
    (:`then`
      (`/Game/Blueprints/BP_JohnGuest.Set Main Menu Mode` _player_ref "/Game/Widgets/WG_Victory.WG_Victory_C"))
    (:`else`)))

(fn `Replay Song`
  (locals (`New Song` :type "SoundBase Object Reference"))
  (bind _lobby_tracks (`self.Lobby Tracks`))
  (bind _output_get (set `local.New Song` (`|GetArrayItem` _lobby_tracks (`KismetMathLibrary.FTrunc` (* (`KismetArrayLibrary.Array_Length` _lobby_tracks) (`KismetMathLibrary.RandomFloat`))))))
  (set `self.Song Time` 0.0)
  (set `self.Song Length` (`SoundBase.Duration` _output_get))
  (for _array_element (`self.Lobby Speakers`)
    (`/Game/Blueprints/BP_LobbySpeaker.Change Song` _array_element _output_get))
  (`self.Set Song Playing` true))

(fn `Roll For Enemy`
  (for _array_element (`self.Enemy Types`)
    (bind (_enemytype _enemycost _enemyspawnchance) (break `/Game/Blueprints/BP_EnemySpawnData` _array_element))
    (if (== (mod (`self.SC Tracker`) (`KismetMathLibrary.Max` _enemycost 1)) 0)
      (if (and (< (`KismetMathLibrary.RandomFloat`) _enemyspawnchance) (<= _enemycost (`self.Spawn Coins`)))
        (`self.Spawn Enemies` _array_element)))))

(fn `Set Song Playing`
  (params (Playing :type Boolean))
  (bind _lobby_speakers (`self.Lobby Speakers`))
  (bind _output_get (set `self.Music Playing` Playing))
  (if _output_get
    (for _array_element _lobby_speakers
      (bind _speaker (`/Game/Blueprints/BP_LobbySpeaker.Speaker` _array_element))
      (`AudioComponent.SetPaused` _speaker false)
      (`AudioComponent.Play` _speaker (`self.Song Time`)))
    (else
      (for _array_element_2 _lobby_speakers
        (`AudioComponent.SetPaused` (`/Game/Blueprints/BP_LobbySpeaker.Speaker` _array_element_2) true)))))

(fn `Song Ended`
  (returns (`Song Ended` :type Boolean))
  (return (>= (`self.Song Time`) (`self.Song Length`))))

(fn `Spawn Enemies`
  (params (`Spawn Data` :type "/Game/Blueprints/BP_EnemySpawnData Structure"))
  (locals (`Enemy Count` :type Integer) (`Cluster Max Dist` :type "Float (double-precision)" :default 2000.0))
  (bind (_enemytype _enemycost) (break `/Game/Blueprints/BP_EnemySpawnData` `Spawn Data`))
  (bind _output_get (set `local.Enemy Count` (+ (`KismetMathLibrary.Max` (`KismetMathLibrary.FTrunc` (* (`KismetMathLibrary.RandomFloat`) (- (/ (`self.Spawn Coins`) (`KismetMathLibrary.Max` _enemycost 1)) 1)))) 1)))
  (bind _rooms (`self.Get Hauntable Cluster` _output_get (`local.Cluster Max Dist`)))
  (for _index (range (`KismetMathLibrary.Min` _output_get (`KismetArrayLibrary.Array_Length` _rooms)))
    (if (>= (`self.Spawn Coins`) _enemycost)
      (bind _success (`self.Spawn Enemy` _enemytype (`|GetArrayItem` _rooms _index)))
      (if _success
        (set `self.Spawn Coins` (- (`self.Spawn Coins`) _enemycost)))
      (else
        (break)))))

(fn `Spawn Enemy`
  (params (`Enemy type` :type "/Game/Blueprints/BP_Enemy Class Reference") (Room :type "/Game/Blueprints/BP_Room Object Reference"))
  (returns (Success :type Boolean))
  (bind _spawn_location (`/Game/Blueprints/BP_Room.Spawn Location` Room))
  (bind (_returnvalue_roll _returnvalue_pitch _returnvalue_yaw) (`KismetMathLibrary.BreakRotator` (`SceneComponent.K2_GetComponentRotation` _spawn_location)))
  (`KismetSystemLibrary.PrintString` (`KismetSystemLibrary.GetClassDisplayName` `Enemy type`))
  (`/Engine/EditorBlueprintResources/StandardMacros.IsValid` Room
    (:`Is Valid`
      (bind _returnvalue (`|SpawnActorFromClass` `Enemy type` (`KismetMathLibrary.MakeTransform` (`SceneComponent.K2_GetComponentLocation` _spawn_location) (`KismetMathLibrary.MakeRotator` 0.0 0.0 _returnvalue_yaw)) "Undefined" "MultiplyWithRoot" null null))
      (bind _success (`/Game/Blueprints/BP_Room.Add Haunter` Room))
      (if _success
        (set `/Game/Blueprints/BP_Enemy.Target Room` Room _returnvalue)
        (`KismetArrayLibrary.Array_Add` (`self.Ghosts`) _returnvalue)
        (else
          (`self.K2_DestroyActor` _returnvalue)))
      (return _success))
    (:`Is Not Valid`
      (return false))))

(fn `Spawn Guests`
  (bind _rooms (`self.Get Random Habitable Room`))
  (bind _spawn_location (`/Game/Blueprints/BP_Room.Spawn Location` _rooms))
  (bind (_returnvalue_roll _returnvalue_pitch _returnvalue_yaw) (`KismetMathLibrary.BreakRotator` (`SceneComponent.K2_GetComponentRotation` _spawn_location)))
  (for _ (range (`self.Guest Count`))
    (`/Engine/EditorBlueprintResources/StandardMacros.IsValid` _rooms
      (:`Is Valid`
        (bind _returnvalue (`|SpawnActorFromClass` "/Game/Blueprints/BP_Guest.BP_Guest_C" (`KismetMathLibrary.MakeTransform` (`SceneComponent.K2_GetComponentLocation` _spawn_location) (`KismetMathLibrary.MakeRotator` 0.0 0.0 _returnvalue_yaw)) "Undefined" "MultiplyWithRoot" null null))
        (bind _success (`/Game/Blueprints/BP_Room.Assign Guest` _rooms _returnvalue))
        (if (not _success)
          (`self.K2_DestroyActor` _returnvalue)
          (else
            (set `/Game/Blueprints/BP_Guest.Lobby` (`BlueprintMapLibrary.Map_Find` (`self.Rooms`) "Lobby") _returnvalue)
            (`KismetArrayLibrary.Array_Add` (`self.Guests`) _returnvalue)
            (set `/Game/Blueprints/BP_Guest.Current Floor` (`KismetStringLibrary.Conv_StringToInt` (`KismetStringLibrary.GetSubstring` (`/Game/Blueprints/BP_Room.Room Name` _rooms))) _returnvalue)))))))

(fn `UserConstructionScript`)