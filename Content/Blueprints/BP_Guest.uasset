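; BP_Guest is a hotel guest that alternates between lobby and assigned room, feeding panic changes into BP_GIGO_GameMode.
; Scares raise panic, flip the destination and start running until a timer, counting down only on arrival, expires.
; Calm guests in the lobby lower panic while music plays, then head to their room after a wait.
; GoToLocation only prints intended moves, Velocity is derived from position deltas, and getters expose disturbance stats.
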(event `self.ReceiveBeginPlay`
  (bind _asbp_gigo_game_mode (cast `/Game/Blueprints/BP_GIGO_GameMode` (`GameplayStatics.GetGameMode`)))
  (set `self.Gamemode Ref` _asbp_gigo_game_mode))

(event `self.ReceiveTick`
  (params (DeltaSeconds :type "Float (single-precision)"))
  (`|ExecutionSequence`
    (:`then_0`
      (if (`self.Can Move`)
        (`self.Go To Location`)))
    (:`then_1`
      (if (> (`self.Panic Timer`) 0.0)
        (set `self.Current Speed` (`self.Run Speed`))
        (if (`self.Arrived`)
          (set `self.Panic Timer` (- (`self.Panic Timer`) DeltaSeconds))
          (set `self.Time In Lobby` 0.0))
        (else
          (set `self.Current Speed` (`self.Walk Speed`))
          (bind _gamemode_ref (`self.Gamemode Ref`)
            (:`then`
              (if (and (`/Game/Blueprints/BP_GIGO_GameMode.Music Playing` _gamemode_ref) (not (`self.Going to Room`)) (`self.Arrived`))
                (`/Game/Blueprints/BP_GIGO_GameMode.Change Panic` _gamemode_ref (* (`self.Calm Strength`) -1.0 DeltaSeconds))
                (bind _output_get (set `self.Time In Lobby` (+ DeltaSeconds (`self.Time In Lobby`))))
                (if (>= _output_get (`self.Wait Time`))
                  (set `self.Going to Room` true))))
            (:`else`)))))
    (:`then_2`
      (`self.Custom Velocity` DeltaSeconds))))

(fn `Arrived`
  (returns (Arrived :type Boolean))
  (if (`self.Going to Room`)
    (bind _room (`self.Room`)
      (:`then`
        (return (`/Game/Blueprints/BP_Room.Guest In Room` _room self)))
      (:`else`
        _))
    (else
      (bind _lobby (`self.Lobby`)
        (:`then`
          (return (`/Game/Blueprints/BP_Room.Guest In Room` _lobby self)))
        (:`else`
          _))))
  (return false))

(fn `Custom Velocity`
  (params (`Delta Seconds` :type "Float (double-precision)"))
  (bind _returnvalue (`SceneComponent.K2_GetComponentLocation` (`self.DefaultSceneRoot`)))
  (set `self.Velocity` (/ (- _returnvalue (`self.Previous Position`)) `Delta Seconds`))
  (set `self.Previous Position` _returnvalue))

(fn `Get Heat`
  (returns (Heat :type "Float (double-precision)"))
  (return (`self.Heat`)))

(fn `Get Locomotiveness`
  (returns (Locomotiveness :type "Float (double-precision)"))
  (return (`self.Max Locomotive Disturbance`)))

(fn `Get Noisiness`
  (returns (Noisiness :type "Float (double-precision)"))
  (return (`self.Noisiness`)))

(fn `Go To Location`
  (bind _gamemode_ref (`self.Gamemode Ref`)
    (:`then`
      (if (not (`self.Arrived`))
        (if (`self.Going to Room`)
          (bind _room (`self.Room`)
            (:`then`
              (if (!= (`/Game/Blueprints/BP_Room.Get Floor` _room) (`self.Current Floor`))
                (bind _output (`|GetArrayItem` (`/Game/Blueprints/BP_GIGO_GameMode.Guest Elevators` _gamemode_ref)))
                (`/Engine/EditorBlueprintResources/StandardMacros.IsValid` _output
                  (:`Is Valid`
                    (`KismetSystemLibrary.PrintString` "Go to elevator!")))
                (else
                  (`KismetSystemLibrary.PrintString` "Go to room!"))))
            (:`else`))
          (else
            (bind _lobby (`self.Lobby`)
              (:`then`
                (if (!= (`/Game/Blueprints/BP_Room.Get Floor` _lobby) (`self.Current Floor`))
                  (`/Engine/EditorBlueprintResources/StandardMacros.IsValid` _output
                    (:`Is Valid`
                      (`KismetSystemLibrary.PrintString` "Go to elevator!")))
                  (else
                    (`KismetSystemLibrary.PrintString` "Go to lobby!"))))
              (:`else`))))))
    (:`else`)))

(fn `Induce Panic`
  (params (`Scare Strength` :type "Float (double-precision)"))
  (set `self.Panic Timer` (`self.Panic Time`))
  (set `self.Going to Room` (not (`self.Going to Room`)))
  (bind _gamemode_ref (`self.Gamemode Ref`)
    (:`then`
      (`/Game/Blueprints/BP_GIGO_GameMode.Change Panic` _gamemode_ref (* (`KismetMathLibrary.FClamp` `Scare Strength`) (`self.Max Panic Amount`))))
    (:`else`)))

(fn `UserConstructionScript`
  (set `self.Current Speed` (`self.Walk Speed`))
  (set `self.Previous Position` (`SceneComponent.K2_GetComponentLocation` (`self.DefaultSceneRoot`))))