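; BP_GIGO_GameInstance tracks the current night and its difficulty, and handles starting nights and returning to the main menu.
; Difficulty comes from a non-negative custom override capped at 10, otherwise from the night's preset, falling back to zero when out of range.
; LoadLevel sets the night unless the previous-night flag is set, then resets BP_GIGO_GameMode.
; LoadMainMenu ends the game through that game mode and switches its player reference into main menu mode.
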(fn `Get Difficulty`
  (returns (Difficulty :type Integer))
  (bind _night_presets (`self.Night Presets`))
  (bind _current_night (`self.Current Night`))
  (if (>= (`self.Custom Difficulty`) 0)
    (return (`KismetMathLibrary.Min` (`self.Custom Difficulty`) 10))
    (elif (and (>= _current_night 0) (< _current_night (`KismetArrayLibrary.Array_Length` _night_presets)))
      (return (`|GetArrayItem` _night_presets _current_night))
      (else
        (return 0)))))

(fn `Load Level`
  (params (Night :type Integer) (`Previous Night` :type Boolean))
  (`|ExecutionSequence`
    (:`then_0`
      (if (not `Previous Night`)
        (set `self.Current Night` Night)))
    (:`then_1`
      (bind _asbp_gigo_game_mode (cast `/Game/Blueprints/BP_GIGO_GameMode` (`GameplayStatics.GetGameMode`)))
      (`/Game/Blueprints/BP_GIGO_GameMode.Reset` _asbp_gigo_game_mode))))

(fn `Load Main Menu`
  (bind _asbp_gigo_game_mode (cast `/Game/Blueprints/BP_GIGO_GameMode` (`GameplayStatics.GetGameMode`)))
  (set `/Game/Blueprints/BP_GIGO_GameMode.Game Started` false _asbp_gigo_game_mode)
  (`/Game/Blueprints/BP_GIGO_GameMode.On End Game` _asbp_gigo_game_mode)
  (bind _player_ref (`/Game/Blueprints/BP_GIGO_GameMode.Player Ref` _asbp_gigo_game_mode)
    (:`then`
      (`/Game/Blueprints/BP_JohnGuest.Set Main Menu Mode` _player_ref "/Game/Widgets/WG_MainMenu.WG_MainMenu_C"))
    (:`else`)))