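; BP_Banshee is a ghost enemy that periodically screams at guests and rooms around it.
; An overlap range gathers targets, and a cooldown timer drains faster while aggroed by occupants in its target room.
; Each scream, also triggered by camera flash, paralyzes John guests, panics other guests, and spawns short-lived room effectors with noisiness scaled by audio falloff distance.
; Defeat plays a vanish animation and sound before delayed destruction.
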(event `self.ReceiveBeginPlay`
  (`parent.ReceiveBeginPlay`))

(event `self.ScreamRange.OnComponentBeginOverlap`
  (params (OverlappedComponent :type "PrimitiveComponent Object Reference") (OtherActor :type "Actor Object Reference") (OtherComp :type "PrimitiveComponent Object Reference") (OtherBodyIndex :type Integer) (bFromSweep :type Boolean) (SweepResult :type "HitResult Structure (by ref)"))
  (bind _targets (`self.Targets`))
  (if (`ActorComponent.ComponentHasTag` OtherComp "Body")
    (bind _asbp_john_guest (cast `/Game/Blueprints/BP_JohnGuest` OtherActor)
      (:`then`
        (`BlueprintSetLibrary.Set_Add` _targets _asbp_john_guest))
      (:`CastFailed`
        (bind _asbp_guest (cast `/Game/Blueprints/BP_Guest` OtherActor))
        (`BlueprintSetLibrary.Set_Add` _targets _asbp_guest)))
    (else
      (bind _asbp_room (cast `/Game/Blueprints/BP_Room` OtherActor))
      (`BlueprintSetLibrary.Set_Add` _targets _asbp_room))))

(event `self.ScreamRange.OnComponentEndOverlap`
  (params (OverlappedComponent :type "PrimitiveComponent Object Reference") (OtherActor :type "Actor Object Reference") (OtherComp :type "PrimitiveComponent Object Reference") (OtherBodyIndex :type Integer))
  (if (`ActorComponent.ComponentHasTag` OtherComp "Body")
    (`BlueprintSetLibrary.Set_Remove` (`self.Targets`) OtherActor)))

(event `self.ReceiveTick`
  (params (DeltaSeconds :type "Float (single-precision)"))
  (`parent.ReceiveTick` DeltaSeconds)
  (if (`self.Alive`)
    (if (<= (`self.ScreamTimer`) 0.0)
      (`self.Scream`)
      (else
        (set `self.ScreamTimer` (- (`self.ScreamTimer`) (* DeltaSeconds (`KismetMathLibrary.SelectFloat` (`self.AggroMultiplier`) 1.0 (`self.Is Aggro`)))))))))

(event `Animate Scream`
  (bind _ghost_skeleton (`self.Ghost Skeleton`))
  (`SkeletalMeshComponent.PlayAnimation` _ghost_skeleton "/Game/Models/Ghosts/Banshee_Character/Animations/Anim_Banshee_Scream.Anim_Banshee_Scream" false)
  (`KismetSystemLibrary.Delay` 4.0)
  (if (`self.Alive`)
    (`SkeletalMeshComponent.PlayAnimation` _ghost_skeleton "/Game/Models/Ghosts/Banshee_Character/Animations/Anim_Banshee_Idle.Anim_Banshee_Idle" true)))

(fn `Determine Aggro`
  (bind _target_room (`self.Target Room`)
    (:`then`
      (if (> (+ (`/Game/Blueprints/BP_Room.Players Present` _target_room) (`/Game/Blueprints/BP_Room.Guests Present` _target_room)) 0)
        (set `self.Is Aggro` true)
        (else
          (set `self.Is Aggro` false))))
    (:`else`)))

(fn `Flash Cam React`
  (`self.Scream`))

(fn `Get Noisiness`
  (returns (Noisiness :type "Float (double-precision)"))
  (return (`self.Noisiness`)))

(fn `On Defeat`
  (bind _ghost_skeleton (`self.Ghost Skeleton`))
  (`SkeletalMeshComponent.Stop` _ghost_skeleton)
  (`SkeletalMeshComponent.PlayAnimation` _ghost_skeleton "/Game/Models/Ghosts/Banshee_Character/Animations/Anim_Banshee_Vanish.Anim_Banshee_Vanish" false)
  (`self.Play Sound` "/Game/Audio/Ghost_Defeat_1.Ghost_Defeat_1")
  (`self.Destroy After Delay` 4.0))

(fn `Scream`
  (bind _audio (`self.Audio`))
  (bind ((`FalloffDistance` _falloffdistance)) (break `SoundAttenuationSettings` (`AudioComponent.AttenuationOverrides` _audio)))
  (set `self.ScreamTimer` (`self.ScreamCooldown`))
  (bind _result (`BlueprintSetLibrary.Set_ToArray` (`self.Targets`)))
  (for _array_element _result
    (bind _asbp_john_guest (cast `/Game/Blueprints/BP_JohnGuest` _array_element)
      (:`then`
        (`/Game/Blueprints/BP_JohnGuest.On Paralyzed` _asbp_john_guest))
      (:`CastFailed`
        (bind _asbp_guest (cast `/Game/Blueprints/BP_Guest` _array_element)
          (:`then`
            (`/Game/Blueprints/BP_Guest.Induce Panic` _asbp_guest 0.25))
          (:`CastFailed`
            (bind _asbp_room (cast `/Game/Blueprints/BP_Room` _array_element))
            (bind (_returnvalue_location _returnvalue_rotation) (`KismetMathLibrary.BreakTransform` (`SceneComponent.K2_GetComponentToWorld` (`/Game/Blueprints/BP_Room.Spawn Location` _asbp_room))))
            (bind _returnvalue (`|SpawnActorFromClass` "/Game/Blueprints/BP_RoomEffector.BP_RoomEffector_C" (`KismetMathLibrary.MakeTransform` _returnvalue_location _returnvalue_rotation) "Undefined" "MultiplyWithRoot" null null))
            (set `/Game/Blueprints/BP_RoomEffector.Noisiness` (* (`self.Noisiness`) (/ (`KismetMathLibrary.FMax` (- _falloffdistance (`KismetMathLibrary.Vector_Distance` _returnvalue_location (`SceneComponent.K2_GetComponentLocation` _audio)))) _falloffdistance)) _returnvalue)
            (set `/Game/Blueprints/BP_RoomEffector.Lifespan` 3.0 _returnvalue))))))
  (`self.Play Sound` "/Game/Audio/Elk_Scream.Elk_Scream")
  (`self.Animate Scream`))

(fn `UserConstructionScript`
  (`parent.UserConstructionScript`)
  (set `self.ScreamTimer` (`self.ScreamCooldown`)))