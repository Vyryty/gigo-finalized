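; Elevator door Blueprint with two sliding panels, LeftDoor and RightDoor, positioned by an open amount.
; The construction script caches each panel's starting relative location.
; SetDoorOpenAmount lerps each panel from its start to a fixed offset in opposite directions along local X.
; It has no timeline or active Tick logic of its own, so the amount must be supplied through that function.
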(event `self.ReceiveTick`
  (params (DeltaSeconds :type "Float (single-precision)")))

(fn `Set Door Open Amount`
  (params (`Amount Open` :type "Float (double-precision)"))
  (bind _left_start (`self.Left Start`))
  (bind _right_start (`self.Right Start`))
  (`SceneComponent.K2_SetRelativeLocation` (`self.Left Door`) (`KismetMathLibrary.VLerp` _left_start (+ _left_start (48.0 0.0 0.0)) `Amount Open`) false false)
  (`SceneComponent.K2_SetRelativeLocation` (`self.Right Door`) (`KismetMathLibrary.VLerp` _right_start (+ _right_start (-48.0 0.0 0.0)) `Amount Open`) false false))

(fn `UserConstructionScript`
  (set `self.Left Start` (`SceneComponent.RelativeLocation` (`self.Left Door`)))
  (set `self.Right Start` (`SceneComponent.RelativeLocation` (`self.Right Door`))))