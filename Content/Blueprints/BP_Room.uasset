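; BP_Room is a room that tracks its players, ghosts, guests and effectors through Body-tagged overlaps.
; Each tick it sums their heat, noisiness and locomotiveness with ambient values, plus a warm-up thermostat, into clamped temperature, noise and movement levels.
; Getters derive hazards and threat level from thresholds, and add time-based Perlin jitter for noisy readings.
; It also caps haunters and assigned guests, and derives its floor from the room name.
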(event `self.ReceiveBeginPlay`
  (bind _asbp_gigo_game_mode (cast `/Game/Blueprints/BP_GIGO_GameMode` (`GameplayStatics.GetGameMode`)))
  (set `self.Gamemode Ref` _asbp_gigo_game_mode))

(event `self.Room Space.OnComponentBeginOverlap`
  (params (OverlappedComponent :type "PrimitiveComponent Object Reference") (OtherActor :type "Actor Object Reference") (OtherComp :type "PrimitiveComponent Object Reference") (OtherBodyIndex :type Integer) (bFromSweep :type Boolean) (SweepResult :type "HitResult Structure (by ref)"))
  (if (`ActorComponent.ComponentHasTag` OtherComp "Body")
    (bind _asbp_john_guest (cast `/Game/Blueprints/BP_JohnGuest` OtherActor)
      (:`then`
        (`BlueprintSetLibrary.Set_Add` (`self.Player Set`) _asbp_john_guest))
      (:`CastFailed`
        (bind _asbp_enemy (cast `/Game/Blueprints/BP_Enemy` OtherActor)
          (:`then`
            (`BlueprintSetLibrary.Set_Add` (`self.Ghost Set`) _asbp_enemy))
          (:`CastFailed`
            (bind _asbp_guest (cast `/Game/Blueprints/BP_Guest` OtherActor)
              (:`then`
                (`BlueprintSetLibrary.Set_Add` (`self.Guest Set`) _asbp_guest))
              (:`CastFailed`
                (bind _asbp_room_effector (cast `/Game/Blueprints/BP_RoomEffector` OtherActor))
                (`BlueprintSetLibrary.Set_Add` (`self.Effector Set`) _asbp_room_effector)))))))))

(event `self.Room Space.OnComponentEndOverlap`
  (params (OverlappedComponent :type "PrimitiveComponent Object Reference") (OtherActor :type "Actor Object Reference") (OtherComp :type "PrimitiveComponent Object Reference") (OtherBodyIndex :type Integer))
  (if (`ActorComponent.ComponentHasTag` OtherComp "Body")
    (bind _asbp_john_guest (cast `/Game/Blueprints/BP_JohnGuest` OtherActor)
      (:`then`
        (`BlueprintSetLibrary.Set_Remove` (`self.Player Set`) _asbp_john_guest))
      (:`CastFailed`
        (bind _asbp_enemy (cast `/Game/Blueprints/BP_Enemy` OtherActor)
          (:`then`
            (`BlueprintSetLibrary.Set_Remove` (`self.Ghost Set`) _asbp_enemy))
          (:`CastFailed`
            (bind _asbp_guest (cast `/Game/Blueprints/BP_Guest` OtherActor)
              (:`then`
                (`BlueprintSetLibrary.Set_Remove` (`self.Guest Set`) _asbp_guest))
              (:`CastFailed`
                (bind _asbp_room_effector (cast `/Game/Blueprints/BP_RoomEffector` OtherActor))
                (`BlueprintSetLibrary.Set_Remove` (`self.Effector Set`) _asbp_room_effector)))))))))

(event `self.ReceiveTick`
  (params (DeltaSeconds :type "Float (single-precision)"))
  (`self.Update Thermostat` DeltaSeconds)
  (`self.Calculate Status`))

(fn `Add Haunter`
  (returns (Success :type Boolean))
  (locals (Result :type Boolean))
  (`|ExecutionSequence`
    (:`then_0`
      (bind _output_get (set `local.Result` (< (`self.Haunter Count`) (`self.Max Ghost Count`))))
      (if _output_get
        (`/Engine/EditorBlueprintResources/StandardMacros.IncrementInt` (`self.Haunter Count`))))
    (:`then_1`
      (return (`local.Result`)))))

(fn `Assign Guest`
  (params (Guest :type "/Game/Blueprints/BP_Guest Object Reference"))
  (returns (Success :type Boolean))
  (locals (Result :type Boolean))
  (bind _assigned_guests (`self.Assigned Guests`))
  (`|ExecutionSequence`
    (:`then_0`
      (if (< (`KismetArrayLibrary.Array_Length` _assigned_guests) (`self.Max Guests`))
        (`KismetArrayLibrary.Array_Add` _assigned_guests Guest)
        (set `/Game/Blueprints/BP_Guest.Room` self Guest)
        (set `local.Result` true)))
    (:`then_1`
      (return (`local.Result`)))))

(fn `Available For Guests`
  (returns (Available :type Boolean))
  (return (< (`KismetArrayLibrary.Array_Length` (`self.Assigned Guests`)) (`self.Max Guests`))))

(fn `Calculate Status`
  (locals (`Temperature Total` :type "Float (double-precision)") (`Noise Total` :type "Float (double-precision)") (`Movement Total` :type "Float (double-precision)") (`Room Effectors` :type "Array of /Game/Blueprints/RoomEffector_I Interface"))
  (bind _room_effectors (`local.Room Effectors`))
  (bind _result (`BlueprintSetLibrary.Set_ToArray` (`self.Player Set`)))
  (for _array_element _result
    (`KismetArrayLibrary.Array_Add` _room_effectors _array_element))
  (bind _result_2 (`BlueprintSetLibrary.Set_ToArray` (`self.Ghost Set`)))
  (for _array_element_2 _result_2
    (`KismetArrayLibrary.Array_Add` _room_effectors _array_element_2))
  (bind _result_3 (`BlueprintSetLibrary.Set_ToArray` (`self.Guest Set`)))
  (for _array_element_3 _result_3
    (`KismetArrayLibrary.Array_Add` _room_effectors _array_element_3))
  (bind _result_4 (`BlueprintSetLibrary.Set_ToArray` (`self.Effector Set`)))
  (for _array_element_4 _result_4
    (`KismetArrayLibrary.Array_Add` _room_effectors _array_element_4))
  (for _array_element_5 _room_effectors
    (bind _heat (`/Game/Blueprints/RoomEffector_I.Get Heat` _array_element_5))
    (set `local.Temperature Total` (+ _heat (`local.Temperature Total`)))
    (bind _noisiness (`/Game/Blueprints/RoomEffector_I.Get Noisiness` _array_element_5))
    (set `local.Noise Total` (+ _noisiness (`local.Noise Total`)))
    (bind _locomotiveness (`/Game/Blueprints/RoomEffector_I.Get Locomotiveness` _array_element_5))
    (set `local.Movement Total` (+ _locomotiveness (`local.Movement Total`))))
  (set `self.Temperature` (`KismetMathLibrary.FClamp` (+ (`local.Temperature Total`) (`self.Ambient Temperature`) (`self.Get Thermostat Temp`))))
  (set `self.Noise` (`KismetMathLibrary.FClamp` (+ (`local.Noise Total`) (`self.Ambient Noise`))))
  (set `self.Movement` (`KismetMathLibrary.FClamp` (+ (`local.Movement Total`) (`self.Ambient Movement`)))))

(fn `Can Haunt`
  (returns (Hauntable :type Boolean))
  (return (< (`self.Haunter Count`) (`self.Max Ghost Count`))))

(fn `Get Floor`
  (returns (Floor :type Integer))
  (return (`KismetMathLibrary.SelectInt` 0 (`KismetStringLibrary.Conv_StringToInt` (`KismetStringLibrary.GetSubstring` (`self.Room Name`))) (== (`self.Room Name`) "Lobby"))))

(fn `Get Movement Dangerous`
  (returns (`Movement Hazard` :type Boolean) (`Hazard Amount` :type "Float (double-precision)"))
  (bind _movement (`self.Movement`))
  (bind _movement_danger_threshold (`self.Movement Danger Threshold`))
  (bind _returnvalue (>= _movement _movement_danger_threshold))
  (return _returnvalue (`KismetMathLibrary.SelectFloat` (/ (- _movement _movement_danger_threshold) (`KismetMathLibrary.FMax` (- 1.0 _movement_danger_threshold) 0.01)) 0.0 _returnvalue)))

(fn `Get Noise Dangerous`
  (returns (`Noise Hazard` :type Boolean) (`Hazard Amount` :type "Float (double-precision)"))
  (bind _noise (`self.Noise`))
  (bind _noise_danger_threshold (`self.Noise Danger Threshold`))
  (bind _returnvalue (>= _noise _noise_danger_threshold))
  (return _returnvalue (`KismetMathLibrary.SelectFloat` (/ (- _noise _noise_danger_threshold) (`KismetMathLibrary.FMax` (- 1.0 _noise_danger_threshold) 0.01)) 0.0 _returnvalue)))

(fn `Get Noisy Movement`
  (returns (Movement :type "Float (double-precision)"))
  (locals (`Random Variance` :type "Float (double-precision)" :default 0.2) (`Random Rate` :type "Float (double-precision)" :default 5.0))
  (return (`KismetMathLibrary.FClamp` (+ (`self.Movement`) (* (- (* (`KismetMathLibrary.PerlinNoise1D` (+ (* (`/Game/Blueprints/BP_GIGO_GameMode.Get Time` (`self.Gamemode Ref`)) (`local.Random Rate`)) (`self.Starting Time Offset`))) 2.0) 1.0) (`local.Random Variance`))))))

(fn `Get Noisy Noise`
  (returns (Noise :type "Float (double-precision)"))
  (locals (`Random Variance` :type "Float (double-precision)" :default 0.1) (`Random Rate` :type "Float (double-precision)" :default 3.0))
  (return (`KismetMathLibrary.FClamp` (+ (`self.Noise`) (* (- (* (`KismetMathLibrary.PerlinNoise1D` (+ (* (`/Game/Blueprints/BP_GIGO_GameMode.Get Time` (`self.Gamemode Ref`)) (`local.Random Rate`)) (`self.Starting Time Offset`))) 2.0) 1.0) (`local.Random Variance`))))))

(fn `Get Noisy Temperature`
  (returns (Noise :type "Float (double-precision)"))
  (locals (`Random Variance` :type "Float (double-precision)" :default 0.05) (`Random Rate` :type "Float (double-precision)" :default 0.125))
  (return (`KismetMathLibrary.FClamp` (+ (`self.Temperature`) (* (- (* (`KismetMathLibrary.PerlinNoise1D` (+ (`self.Starting Time Offset`) (* (`/Game/Blueprints/BP_GIGO_GameMode.Get Time` (`self.Gamemode Ref`)) (`local.Random Rate`)))) 2.0) 1.0) (`local.Random Variance`))))))

(fn `Get Temperature Dangerous`
  (returns (`Temp Hazard` :type Boolean) (`Hazard Amount` :type "Float (double-precision)"))
  (bind _temperature (`self.Temperature`))
  (bind _temp_danger_threshold (`self.Temp Danger Threshold`))
  (bind _returnvalue (>= _temperature _temp_danger_threshold))
  (return _returnvalue (`KismetMathLibrary.SelectFloat` (/ (- _temperature _temp_danger_threshold) (`KismetMathLibrary.FMax` (- 1.0 _temp_danger_threshold) 0.01)) 0.0 _returnvalue)))

(fn `Get Thermostat Temp`
  (returns (`Current Thermostat Temp` :type "Float (double-precision)"))
  (return (* (`self.Thermostat Temp`) (/ (`self.Thermostat Warmup Timer`) (`KismetMathLibrary.FMax` (`self.Thermostat Warmup Time`) 0.01)))))

(fn `Get Threat Level`
  (returns (`Threat Level` :type String) (`Threat Color` :type "Color Structure"))
  (locals (`Threat Levels` :type "Map of String to Color Structure") (`Curr Threat` :type Integer))
  (bind _threat_levels (`local.Threat Levels`))
  (bind _curr_threat (`local.Curr Threat`))
  (`|ExecutionSequence`
    (:`then_0`
      (if (`self.Get Temperature Dangerous`)
        (`/Engine/EditorBlueprintResources/StandardMacros.IncrementInt` _curr_threat)))
    (:`then_1`
      (if (`self.Get Noise Dangerous`)
        (`/Engine/EditorBlueprintResources/StandardMacros.IncrementInt` _curr_threat)))
    (:`then_2`
      (if (`self.Get Movement Dangerous`)
        (`/Engine/EditorBlueprintResources/StandardMacros.IncrementInt` _curr_threat)))
    (:`then_3`
      (bind _keys (`BlueprintMapLibrary.Map_Keys` _threat_levels))
      (bind _output (`|GetArrayItem` _keys _curr_threat))
      (return _output (`BlueprintMapLibrary.Map_Find` _threat_levels _output)))))

(fn `Ghosts Present`
  (returns (`Ghost Count` :type Integer))
  (return (`BlueprintSetLibrary.Set_Length` (`self.Ghost Set`))))

(fn `Guest In Room`
  (params (Guest :type "/Game/Blueprints/BP_Guest Object Reference"))
  (returns (`Guest Present` :type Boolean))
  (return (`BlueprintSetLibrary.Set_Contains` (`self.Guest Set`) Guest)))

(fn `Guests Present`
  (returns (`Guest Count` :type Integer))
  (return (`BlueprintSetLibrary.Set_Length` (`self.Guest Set`))))

(fn `Players Present`
  (returns (`Player Count` :type Integer))
  (return (`BlueprintSetLibrary.Set_Length` (`self.Player Set`))))

(fn `Remove Haunter`
  (if (> (`self.Haunter Count`) 0)
    (`/Engine/EditorBlueprintResources/StandardMacros.DecrementInt` (`self.Haunter Count`))))

(fn `Update Thermostat`
  (params (`Delta Seconds` :type "Float (double-precision)"))
  (set `self.Thermostat Warmup Timer` (`KismetMathLibrary.FClamp` (+ (`self.Thermostat Warmup Timer`) (`KismetMathLibrary.SelectFloat` `Delta Seconds` (* `Delta Seconds` -1.0) (`self.Heated`))) 0.0 (`self.Thermostat Warmup Time`))))

(fn `UserConstructionScript`
  (set `self.Starting Time Offset` (* (`KismetMathLibrary.RandomFloat`) (`KismetMathLibrary.GetPI`) 2.0)))