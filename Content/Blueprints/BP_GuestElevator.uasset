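; Guest elevator actor that travels between preset floor locations to serve queued calls, with a guest capacity check and wait-location lookup.
; CallElevator sorts requests into up and down queues relative to the current floor.
; Tick moves it toward the floor picked from GoingUp and queue searches (both read UpQueue), then snaps, stops and dequeues on arrival.
; DoorSensor overlaps track the current door; nothing here clears Stopped or changes GoingUp.
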(event `self.ReceiveTick`
  (params (DeltaSeconds :type "Float (single-precision)"))
  (set `self.Current Floor` (`self.Nearest Floor` true))
  (if (not (`self.Stopped`))
    (`self.Move` DeltaSeconds)))

(event `self.Door Sensor.OnComponentBeginOverlap`
  (params (OverlappedComponent :type "PrimitiveComponent Object Reference") (OtherActor :type "Actor Object Reference") (OtherComp :type "PrimitiveComponent Object Reference") (OtherBodyIndex :type Integer) (bFromSweep :type Boolean) (SweepResult :type "HitResult Structure (by ref)"))
  (bind _asbp_elevator_door (cast `/Game/Blueprints/BP_ElevatorDoor` OtherActor))
  (set `self.Door` _asbp_elevator_door))

(event `self.Door Sensor.OnComponentEndOverlap`
  (params (OverlappedComponent :type "PrimitiveComponent Object Reference") (OtherActor :type "Actor Object Reference") (OtherComp :type "PrimitiveComponent Object Reference") (OtherBodyIndex :type Integer))
  (if (== OtherActor (`self.Door`))
    (set `self.Door` null)))

(fn `Call Elevator`
  (params (Floor :type Integer))
  (if (`self.On Floor` Floor)
    _
    (elif (> Floor (`self.Current Floor`))
      (`BlueprintSetLibrary.Set_Add` (`self.Up Queue`) Floor)
      (else
        (`BlueprintSetLibrary.Set_Add` (`self.Down Queue`) Floor)))))

(fn `Can Fit`
  (returns (`Can Fit` :type Boolean))
  (return (< (`BlueprintSetLibrary.Set_Length` (`self.Guests`)) (`self.Max Capacity`))))

(fn `Finish Queue`
  (returns (Finished :type Boolean))
  (bind _going_up (`self.Going Up`))
  (return (or (and _going_up (<= (`BlueprintSetLibrary.Set_Length` (`self.Up Queue`)) 0)) (and (not _going_up) (<= (`BlueprintSetLibrary.Set_Length` (`self.Down Queue`)) 0)))))

(fn `Get Next Floor`
  (returns (Floor :type Integer))
  (if (`self.Finish Queue`)
    (return (`self.Nearest Floor` false))
    (else
      (return (`KismetMathLibrary.SelectInt` (`self.Nearest Higher Floor`) (`self.Nearest Lower Floor`) (`self.Going Up`))))))

(fn `Get Wait Location`
  (params (Floor :type Integer))
  (returns (`Wait Location` :type "Vector Structure"))
  (bind _wait_area (`self.Wait Area`))
  (return (+ (`|GetArrayItem` (`self.Floor Locations`) Floor) (* (`SceneComponent.GetForwardVector` _wait_area) (`ArrowComponent.ArrowLength` _wait_area)))))

(fn `Move`
  (params (`Delta Seconds` :type "Float (double-precision)"))
  (locals (`Close Enough Threshold` :type "Float (double-precision)" :default 25.0))
  (bind _nearest_floor (`self.Nearest Floor` true))
  (bind _wait_area (`self.Wait Area`))
  (bind _close_enough_threshold (`local.Close Enough Threshold`))
  (bind _defaultsceneroot (`self.DefaultSceneRoot`))
  (bind _returnvalue (`SceneComponent.K2_GetComponentLocation` _defaultsceneroot))
  (bind _output (`|GetArrayItem` (`self.Floor Locations`) (`self.Get Next Floor`)))
  (bind _returnvalue_2 (* `Delta Seconds` (`self.Speed`)))
  (bind _relativelocation (`SceneComponent.RelativeLocation` _wait_area))
  (bind _returnvalue_3 (- (+ _output _relativelocation) _returnvalue))
  (bind _returnvalue_4 (`KismetMathLibrary.VSizeSquared` _returnvalue_3))
  (if (and (not (`self.Stopped`)) (or (> (`BlueprintSetLibrary.Set_Length` (`self.Up Queue`)) 0) (> (`BlueprintSetLibrary.Set_Length` (`self.Down Queue`)) 0)))
    (if (<= (`KismetMathLibrary.Vector_DistanceSquared` (`SceneComponent.K2_GetComponentLocation` _wait_area) _output) _close_enough_threshold)
      (`SceneComponent.K2_SetWorldLocation` _defaultsceneroot (+ _output _relativelocation) false false)
      (set `self.Stopped` true)
      (if (`self.Going Up`)
        (`BlueprintSetLibrary.Set_Remove` (`self.Up Queue`) _nearest_floor)
        (else
          (`BlueprintSetLibrary.Set_Remove` (`self.Down Queue`) _nearest_floor)))
      (else
        (`SceneComponent.K2_SetWorldLocation` _defaultsceneroot (+ _returnvalue (* (`KismetMathLibrary.Normal` _returnvalue_3) (`KismetMathLibrary.SelectFloat` _returnvalue_2 (`KismetMathLibrary.Sqrt` _returnvalue_4) (> (- _returnvalue_4 (* _returnvalue_2 _returnvalue_2)) _close_enough_threshold)))) false false)))))

(fn `Nearest Floor`
  (params (`Include Current` :type Boolean))
  (returns (`Nearest Floor` :type Integer))
  (locals (`Lower Floor` :type Integer) (`Higher Floor` :type Integer) (Result :type Integer) (`Smallest Distance` :type "Float (double-precision)"))
  (bind _current_floor (`self.Current Floor`))
  (bind _floor_locations (`self.Floor Locations`))
  (bind _smallest_distance (`local.Smallest Distance`))
  (bind _returnvalue (`SceneComponent.K2_GetComponentLocation` (`self.Wait Area`)))
  (bind _returnvalue_2 (`KismetMathLibrary.Vector_DistanceSquared` _returnvalue (`|GetArrayItem` _floor_locations (`local.Lower Floor`))))
  (bind _output_get (set `local.Lower Floor` (`self.Nearest Lower Floor`)))
  (set `local.Higher Floor` (`self.Nearest Higher Floor`))
  (set `local.Result` (`KismetMathLibrary.SelectInt` _current_floor _output_get `Include Current`))
  (set `local.Smallest Distance` (`KismetMathLibrary.SelectFloat` (`KismetMathLibrary.Vector_DistanceSquared` _returnvalue (`|GetArrayItem` _floor_locations _current_floor)) _returnvalue_2 `Include Current`))
  (`|ExecutionSequence`
    (:`then_0`
      (if (< _smallest_distance _returnvalue_2)
        (set `local.Smallest Distance` _returnvalue_2)
        (set `local.Result` (`local.Lower Floor`))))
    (:`then_1`
      (if (or (< _smallest_distance (`KismetMathLibrary.Vector_DistanceSquared` _returnvalue (`|GetArrayItem` _floor_locations (`local.Higher Floor`)))) (and (not `Include Current`) (== (`self.Current Floor`) (`local.Lower Floor`))))
        (set `local.Result` (`local.Higher Floor`))))
    (:`then_2`
      (return (`local.Result`)))))

(fn `Nearest Higher Floor`
  (returns (Floor :type Integer))
  (locals (`Nearest Floor` :type Integer) (`Nearest Distance` :type Integer))
  (bind _up_queue (`self.Up Queue`))
  (set `local.Nearest Floor` (`self.Current Floor`))
  (set `local.Nearest Distance` (`KismetArrayLibrary.Array_Length` (`self.Floor Locations`)))
  (`|ExecutionSequence`
    (:`then_0`
      (if (> (`BlueprintSetLibrary.Set_Length` _up_queue) 0)
        (bind _result (`BlueprintSetLibrary.Set_ToArray` _up_queue))
        (for _array_element _result
          (bind _returnvalue (- _array_element (`local.Nearest Floor`)))
          (if (< _returnvalue (`local.Nearest Distance`))
            (set `local.Nearest Floor` _array_element)
            (set `local.Nearest Distance` _returnvalue)))))
    (:`then_1`
      (return (`local.Nearest Floor`)))))

(fn `Nearest Lower Floor`
  (returns (Floor :type Integer))
  (locals (`Nearest Floor` :type Integer) (`Nearest Distance` :type Integer))
  (bind _up_queue (`self.Up Queue`))
  (set `local.Nearest Floor` (`self.Current Floor`))
  (set `local.Nearest Distance` (`KismetArrayLibrary.Array_Length` (`self.Floor Locations`)))
  (`|ExecutionSequence`
    (:`then_0`
      (if (> (`BlueprintSetLibrary.Set_Length` _up_queue) 0)
        (bind _result (`BlueprintSetLibrary.Set_ToArray` _up_queue))
        (for _array_element _result
          (bind _returnvalue (- (`local.Nearest Floor`) _array_element))
          (if (< _returnvalue (`local.Nearest Distance`))
            (set `local.Nearest Floor` _array_element)
            (set `local.Nearest Distance` _returnvalue)))))
    (:`then_1`
      (return (`local.Nearest Floor`)))))

(fn `On Floor`
  (params (Floor :type Integer))
  (returns (`On Floor` :type Boolean))
  (return (and (== Floor (`self.Current Floor`)) (`self.Stopped`))))

(fn `UserConstructionScript`)