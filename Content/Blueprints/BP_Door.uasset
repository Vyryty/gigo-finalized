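; BP_Door is an interactable door that swings open away from or toward either side and closes itself after a delay.
; Interact closes an open door, or picks the swing direction from the interactor's side using a dot product with the frame mesh's right vector.
; A timeline drives the rotation, reverses to close, and toggles IsOpen on finishing.
; The construction script sets the door as the highlight mesh.
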(event `OpenDoor`
  (bind (_direction _doorrotate) (`Timeline|doorMoving` :!label _label)
    (:`Update`
      (`SceneComponent.K2_SetRelativeRotation` (`self.Door`) (`|EaseFunction` "Linear" _doorrotate (struct) (`self.LastOpen`)) false false))
    (:`Finished`
      (bind _output_get (set `self.IsOpen` (not (`self.IsOpen`))))
      (if _output_get
        (`KismetSystemLibrary.Delay` 10.0)
        (if _output_get
          (`self.CloseDoor`))))))

(event `CloseDoor`
  (goto _label :!via `Reverse`))

(fn `Interact`
  (params (Interactor :type "Actor Object Reference"))
  (returns (Success :type Boolean))
  (bind _staticmesh (`self.StaticMesh`))
  (if (`self.IsOpen`)
    (`self.CloseDoor`)
    (else
      (set `self.LastOpen` (`KismetMathLibrary.SelectRotator` (struct :`Yaw` -90.0) (struct :`Yaw` 90.0) (> (`KismetMathLibrary.Dot_VectorVector` (- (`self.K2_GetActorLocation` Interactor) (`SceneComponent.K2_GetComponentLocation` _staticmesh)) (`SceneComponent.GetRightVector` _staticmesh)) 0.0)))
      (`self.OpenDoor`)))
  (return true))

(fn `UserConstructionScript`
  (`parent.UserConstructionScript`)
  (set `self.Highlight Mesh` (`self.Door`)))